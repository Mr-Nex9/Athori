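; Player controller for a chess game that shows the mouse cursor and forwards mouse input to the Board actor.
; It caches the first Board found at BeginPlay.
; Left-click release passes the hit location under the cursor from a Visibility trace to the board, while right-click release calls its right-click handler.
; Its ActorBeginCursorOver event sends the same traced location for pawn highlighting.
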(event EventBeginPlay
  (Variables|Default|SetbShowMouseCursor true)
  (bind _outactors (Actor|GetAllActorsOfClass "/Game/Aleian_Chess/Blueprints/Board.Board_C"))
  (Variables|Default|SetBoard_C (Utilities|Array|Get(acopy) _outactors)))

(event EventTick
  (params (DeltaSeconds :type Float%20%28single-precision%29)))

(event MouseInput|EventActorBeginCursorOver
  (Default|HighlightHoveredPawn (Variables|Default|GetBoard_C) (.Location (Collision|BreakHitResult (.HitResult (Game|Player|GetHitResultUnderCursorbyChannel "TraceTypeQuery1" true))))))

(event Input|MouseEvents|LeftMouseButton
  (params (Key :type Key%20Structure :default "None"))
  (:Released
    (Default|OnLeftClick (Variables|Default|GetBoard_C) (.Location (Collision|BreakHitResult (.HitResult (Game|Player|GetHitResultUnderCursorbyChannel "TraceTypeQuery1" true)))))))

(event Input|MouseEvents|RightMouseButton
  (params (Key :type Key%20Structure :default "None"))
  (:Released
    (Default|OnRightClick (Variables|Default|GetBoard_C))))

(fn ConstructionScript)