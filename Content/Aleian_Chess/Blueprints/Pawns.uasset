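; Pawns Blueprint that spawns the chess pieces and walls for Aleian Chess as static mesh components added to the Board actor.
; PlacePawns picks each piece from a start-position table and applies team rotation and material, while SinglePawnSpawn places a chosen piece type at a given index.
; CreateWall adds rotated, mossy segments along an index path.
; PawnsMesh tracks components by square, with indices converted to positions on a nine-wide grid.
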(fn ConstructionScript)

(fn PlacePawns
  (params (Index :type Integer) (Cur_team :type Integer))
  (Development|PrintString "Placing Pawns" false)
  (Utilities|SetBoard)
  (LocalVariables|SetCur_pos Index)
  (bind _output_get (LocalVariables|SetCur_teamm Cur_team))
  (switch int _output_get
    (:1
      (LocalVariables|SetRotation "0.000000,-90.000000,0.000000"))
    (:2
      (LocalVariables|SetRotation "0.000000,90.000000,0.000000")))
  ;[1 1 1] Determining which piece based on board index
  (bind _output_get_2 (Variables|Default|SetPawnType (Utilities|Select :Index (Utilities|Array|Get(acopy) (Variables|Default|GetPieces_start_position) (LocalVariables|GetCur_pos)) :Option%200 0 :Option%201 "/Game/Aleian_Chess/Objects/Actuals/Footmen.Footmen" :Option%202 "/Game/Aleian_Chess/Objects/Actuals/Mage.Mage" :Option%203 "/Game/Aleian_Chess/Objects/Actuals/Captain.Captain" :Option%204 "/Game/Aleian_Chess/Objects/Actuals/General2.General2" :Option%205 "/Game/Aleian_Chess/Objects/Actuals/King2.King2")))
  ;[1 1 1] Check if there is a pawn to create
  (if (!= _output_get_2 0)
    ;[1 1 1] Create piece based on starting location and place on board
    (bind _returnvalue (AddComponent|AddStaticMeshComponent (Variables|Default|GetBoard_C) false (|ScalePawn)))
    (bind _output_get_3 (LocalVariables|SetCurrent_Pawn _returnvalue))
    (Components|StaticMesh|SetStaticMesh _output_get_3 (Variables|Default|GetPawnType))
    ;;[1 1 1] Add piece to array
    (Utilities|Array|Add (Variables|Default|GetPawns_Mesh) (LocalVariables|GetCurrent_Pawn))
    (Rendering|Material|SetMaterial (LocalVariables|GetCurrent_Pawn) 0 (Utilities|Select :Index (LocalVariables|GetCur_teamm) :Option%200 0 :Option%201 (Variables|Default|GetArmy1_Material) :Option%202 (Variables|Default|GetArmy2_Material)))
    (return (LocalVariables|GetCur_pos) (Utilities|GetDisplayName (Variables|Default|GetPawnType)))
    (else
      ;[1 1 1] If no, Add empty slot to array
      (Utilities|Array|Add (Variables|Default|GetPawns_Mesh) 0)
      (Development|PrintString "No Pawns Placed" false)
      (return (LocalVariables|GetCur_pos) (Utilities|GetDisplayName (Variables|Default|GetPawnType))))))

(fn SinglePawnSpawn
  (params (Cur_team :type Integer) (Type :type String) (Index :type Integer))
  (Development|PrintString "Placing Pawns" false false)
  (Utilities|SetBoard)
  (LocalVariables|SetCur_teamm Cur_team)
  (switch string Type
    (:Mage
      (Variables|Default|SetPawnType "/Game/Aleian_Chess/Objects/Actuals/Mage.Mage"))
    (:Captain
      (Variables|Default|SetPawnType "/Game/Aleian_Chess/Objects/Actuals/Captain.Captain"))
    (:General
      (Variables|Default|SetPawnType "/Game/Aleian_Chess/Objects/Actuals/General2.General2"))
    (:King
      (Variables|Default|SetPawnType "/Game/Aleian_Chess/Objects/Actuals/King2.King2"))
    (:Knight
      (Variables|Default|SetPawnType "/Game/Aleian_Chess/Objects/Actuals/Knight.Knight"))
    (:Archmage
      (Variables|Default|SetPawnType "/Game/Aleian_Chess/Objects/Actuals/Archmage.Archmage"))
    (:Footmen
      (Variables|Default|SetPawnType "/Game/Aleian_Chess/Objects/Actuals/Footmen.Footmen")))
  (LocalVariables|SetCur_pos Index)
  ;[1 1 1] Place new static mesh based on Pawn type
  (bind _returnvalue (AddComponent|AddStaticMeshComponent (Variables|Default|GetBoard_C) false (|ScaleandPositionPawn)))
  (bind _output_get (LocalVariables|SetCurrent_Pawn _returnvalue))
  (Components|StaticMesh|SetStaticMesh _output_get (Variables|Default|GetPawnType))
  ;;[1 1 1] Update Array
  (Utilities|Array|SetArrayElem (Variables|Default|GetPawns_Mesh) (LocalVariables|GetCur_pos) (LocalVariables|GetCurrent_Pawn) true)
  ;[1 1 1] Set color based on which team
  (Rendering|Material|SetMaterial (LocalVariables|GetCurrent_Pawn) 0 (Utilities|Select :Index (LocalVariables|GetCur_teamm) :Option%200 0 :Option%201 (Variables|Default|GetArmy1_Material) :Option%202 (Variables|Default|GetArmy2_Material)))
  (return))

(fn CreateWall
  (params (Direction :type Float%20%28double-precision%29) (Wall%20Path :type Array%20of%20Integers))
  (bind _output_get (LocalVariables|SetRotation Direction))
  (if (== _output_get 0.0)
    (LocalVariables|SetPlacement "-200.000000,0.000000,0.000000")
    (else
      (LocalVariables|SetPlacement "0.000000,-200.000000,0.000000")))
  (for _array_element Wall%20Path
    (bind _output_get_2 (LocalVariables|SetCur_index _array_element))
    (bind _returnvalue (AddComponent|AddStaticMeshComponent (Variables|Default|GetBoard_C) false (Math|Transform|MakeTransform (.location (Math|Conversions|ToTransform(Vector) (+ (Utilities|IndextoPosition _output_get_2) (LocalVariables|GetPlacement)))) (Math|Rotator|MakeRotator (.Roll (Math|Rotator|BreakRotator (.rotation (Math|Conversions|ToTransform(Vector) (+ (Utilities|IndextoPosition _output_get_2) (LocalVariables|GetPlacement)))))) (.Pitch (Math|Rotator|BreakRotator (.rotation (Math|Conversions|ToTransform(Vector) (+ (Utilities|IndextoPosition _output_get_2) (LocalVariables|GetPlacement)))))) (+ (.Yaw (Math|Rotator|BreakRotator (.rotation (Math|Conversions|ToTransform(Vector) (+ (Utilities|IndextoPosition _output_get_2) (LocalVariables|GetPlacement)))))) (LocalVariables|GetRotation))) "1.000000,1.000000,1.000000")))
    (Rendering|Material|SetMaterial _returnvalue 0 "/Game/StarterContent/Materials/M_Ground_Moss.M_Ground_Moss")
    (Utilities|Array|SetArrayElem (Variables|Default|GetPawns_Mesh) (LocalVariables|GetCur_index) _returnvalue))
  (return))